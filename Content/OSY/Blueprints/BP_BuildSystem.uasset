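; Build-mode component for OSY_TESTCharacter that lets the player preview, rotate and place BP_BuildMaster actors.
; While build mode is toggled on, Tick line-traces from the player camera and moves a collision-free cube preview mesh, created once via a resettable DoOnce, to the hit point.
; Holding the rotate input runs a looping timer that increments the preview rotation.
; Placing spawns the actor at the preview transform and exits build mode.
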(event `self.ReceiveBeginPlay`
  (bind _asosy_testcharacter (cast `OSY_TESTCharacter` (`self.GetOwner`)))
  (set `self.As OSY TESTCharacter` _asosy_testcharacter)
  (set `self.Player Cam` (`OSY_TESTCharacter.playerCam` _asosy_testcharacter)))

(event `self.ReceiveTick`
  (params (DeltaSeconds :type "Float (single-precision)"))
  (if (`self.inBuildMode`)
    (`self.PreviweLoop`)))

(event `PreviweLoop`
  (bind (_returnvalue_location _returnvalue_rotation) (`KismetMathLibrary.BreakTransform` (`SceneComponent.K2_GetComponentToWorld` (`self.Player Cam`))))
  (bind (_outhit _returnvalue) (`KismetSystemLibrary.LineTraceSingle` _returnvalue_location (+ _returnvalue_location (* (`KismetMathLibrary.GetForwardVector` _returnvalue_rotation) 2000.0)) "TraceTypeQuery1"))
  (if _returnvalue
    (`|ExecutionSequence`
      (:`then_0`
        (`/Engine/EditorBlueprintResources/StandardMacros.DoOnce` false :!label _label
          (:`Completed`
            (bind _returnvalue_2 (`|AddComponentByClass` (`self.As OSY TESTCharacter`) "/Script/Engine.StaticMeshComponent" false (`self.Build Priview Transform`)))
            (bind _output_get (set `self.Preview Mesh` _returnvalue_2))
            (`StaticMeshComponent.SetStaticMesh` _output_get "/Engine/EngineMeshes/Cube.Cube")
            (`PrimitiveComponent.SetMaterial` (`self.Preview Mesh`) 0 "/Game/MetaHumans/OSY/Nasim/M-BuildPreview.M-BuildPreview")
            (`PrimitiveComponent.SetCollisionEnabled` (`self.Preview Mesh`) "NoCollision"))))
      (:`then_1`
        (bind _output_get_2 (set `self.Build Priview Transform` (`KismetMathLibrary.MakeTransform` (`.Location` (`GameplayStatics.BreakHitResult` _outhit)) (`self.BuildPreviewRotation`))))
        (`SceneComponent.K2_SetWorldTransform` (`self.Preview Mesh`) _output_get_2 false false)))))

(event `Reset build Mode`
  (goto _label :!via `Reset`))

(event `EnhancedInput|/Game/OSY/Inputs/IA_OSY_Build`
  (params (ActionValue :type Boolean) (ElapsedSeconds :type "Float (double-precision)") (TriggeredSeconds :type "Float (double-precision)") (InputAction :type "InputAction Object Reference" :default "/Game/OSY/Inputs/IA_OSY_Build.IA_OSY_Build"))
  (:`Started`
    (if (not (`self.inBuildMode`))
      (set `self.inBuildMode` true)
      (else
        (set `self.inBuildMode` false :!label _label_2)
        (bind _preview_mesh (`self.Preview Mesh`)
          (:`then`
            (`StaticMeshComponent.SetStaticMesh` _preview_mesh null)
            (set `self.Preview Mesh` null)
            (`self.Reset build Mode`))
          (:`else`))))))

(event `StopBuildMode`
  (goto _label_2))

(event `EnhancedInput|/Game/OSY/Inputs/IA_OSY_PlaceBuild`
  (params (ActionValue :type Boolean) (ElapsedSeconds :type "Float (double-precision)") (TriggeredSeconds :type "Float (double-precision)") (InputAction :type "InputAction Object Reference" :default "/Game/OSY/Inputs/IA_OSY_PlaceBuild.IA_OSY_PlaceBuild"))
  (:`Triggered`
    (if (`self.inBuildMode`)
      (`|SpawnActorFromClass` "/Game/OSY/Blueprints/BP_BuildMaster.BP_BuildMaster_C" (`self.Build Priview Transform`) "AlwaysSpawn" "MultiplyWithRoot" null null)
      (`self.StopBuildMode`))))

(event `EnhancedInput|/Game/OSY/Inputs/IA_OSY_RotaionBuild`
  (params (ActionValue :type Boolean) (ElapsedSeconds :type "Float (double-precision)") (TriggeredSeconds :type "Float (double-precision)") (InputAction :type "InputAction Object Reference" :default "/Game/OSY/Inputs/IA_OSY_RotaionBuild.IA_OSY_RotaionBuild"))
  (:`Started`
    (bind _returnvalue (`KismetSystemLibrary.K2_SetTimerDelegate` (delegate `Rotate Preview`) 0.01 true))
    (set `self.Rotate Build Preview Loop` _returnvalue))
  (:`Completed`
    (`KismetSystemLibrary.K2_ClearAndInvalidateTimerHandle` (`self.Rotate Build Preview Loop`))
    (set `self.Rotate Build Preview Loop` (struct))))

(event `Rotate Preview`
  (bind (_build_priview_transform_location _build_priview_transform_rotation) (`KismetMathLibrary.BreakTransform` (`self.Build Priview Transform`)))
  (set `self.BuildPreviewRotation` (`KismetMathLibrary.ComposeRotators` _build_priview_transform_rotation (struct :`Yaw` 5.0))))