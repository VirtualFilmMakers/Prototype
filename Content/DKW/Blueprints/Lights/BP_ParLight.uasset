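; BP_ParLight is a controllable par stage light with a pan/tilt head joint and a spotlight.
; On BeginPlay or OpenAssetPanel it creates a BP_ParLightWidget, passes it the light and joint, and seeds its sliders from current values.
; Tick reapplies stored rotation, intensity and cone angle variables, while drawing owner and network role debug text.
; Server and multicast parameter events are empty stubs, as is closing the panel.
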(event `self.ReceiveBeginPlay`
  (`self.OpenControlWidget`))

(event `self.OpenAssetPanel`
  (params (AssetWithControlPanel :type "Actor Object Reference"))
  (`self.OpenControlWidget`))

(event `self.CloseAssetPanel`
  (params (AssetWithControlPanel :type "Actor Object Reference"))
  (if true
    _))

(event `self.ReceiveActorOnClicked`
  (params (ButtonPressed :type "Key Structure"))
  (`KismetSystemLibrary.PrintString` "Hello"))

(event `self.ReceiveTick`
  (params (DeltaSeconds :type "Float (single-precision)"))
  (bind _intensiy (`self.Intensiy`))
  (bind _spotlight (`self.SpotLight`))
  (`self.NetDebug`)
  (`|ExecutionSequence`
    (:`then_0`
      (`SceneComponent.K2_SetRelativeRotation` (`self.headJoint`) (`self.HeadRotation`) false false))
    (:`then_1`
      (`LightComponent.SetIntensity` _spotlight _intensiy))
    (:`then_2`
      (`SpotLightComponent.SetInnerConeAngle` _spotlight (`self.InnerConeAnle`)))
    (:`then_3`
      (`SpotLightComponent.SetOuterConeAngle` _spotlight (`self.OuterConeAngle`))
      (`KismetSystemLibrary.PrintString` (`KismetStringLibrary.Concat_StrStr` "intensity | " (`KismetStringLibrary.Conv_DoubleToString` _intensiy))))))

(event `ServerUpdateParam`)

(event `MulticastParams`)

(fn `NetDebug`
  (bind _returnvalue (`self.K2_GetActorLocation`))
  (bind _returnvalue_2 (+ _returnvalue (0.0 0.0 -10.0)))
  ;[1 1 1] Comment
  (`KismetSystemLibrary.DrawDebugString` _returnvalue (`KismetStringLibrary.Concat_StrStr` "Owner" (`KismetSystemLibrary.GetDisplayName` (`self.GetOwner`))) null)
  (`KismetSystemLibrary.DrawDebugString` _returnvalue_2 (`KismetStringLibrary.Concat_StrStr` "Local Role" (`|GetEnumeratorNameAsString` (`self.GetLocalRole`))) null)
  (`KismetSystemLibrary.DrawDebugString` (+ _returnvalue_2 (0.0 0.0 -10.0)) (`KismetStringLibrary.Concat_StrStr` "Remote Role" (`|GetEnumeratorNameAsString` (`self.GetRemoteRole`))) null))

(fn `OpenControlWidget`
  (bind _returnvalue (`|CreateWidget` "/Game/DKW/UI/Light/BP_ParLightWidget.BP_ParLightWidget_C"))
  ;[1 1 1] create widget
  (set `self.ControlWidget` _returnvalue)
  (`UserWidget.AddToViewport` _returnvalue 0)
  (`UserWidget.SetPositionInViewport` _returnvalue (1600.0 50.0) true)
  ;[1 1 1] Set references
  (`|ExecutionSequence`
    (:`then_0`
      (set `/Game/DKW/UI/Light/BP_ParLightWidget.linkedAsset` self _returnvalue))
    (:`then_1`
      (set `/Game/DKW/UI/Light/BP_ParLightWidget.Light Source` (`self.SpotLight`) _returnvalue))
    (:`then_2`
      (set `/Game/DKW/UI/Light/BP_ParLightWidget.headJoint` (`self.headJoint`) _returnvalue))
    (:`then_3`
      ;[1 1 1] Set Default UI value
      (`self.SetDefaultUIValue`))))

(fn `SetDefaultUIValue`
  (bind _spotlight (`self.SpotLight`))
  (bind (_relativerotation_roll _relativerotation_pitch _relativerotation_yaw) (`KismetMathLibrary.BreakRotator` (`SceneComponent.RelativeRotation` (`self.headJoint`))))
  (bind _asbp_par_light_widget (cast `/Game/DKW/UI/Light/BP_ParLightWidget` (`self.ControlWidget`)))
  (`|ExecutionSequence`
    (:`then_1`
      (`/Game/DKW/UI/Module/BP_SliderModule.SetSliderValue` (`/Game/DKW/UI/Light/BP_ParLightWidget.BP_SliderModule_Intensity` _asbp_par_light_widget) (`LightComponentBase.Intensity` _spotlight)))
    (:`then_2`
      (`/Game/DKW/UI/Module/BP_SliderModule.SetSliderValue` (`/Game/DKW/UI/Light/BP_ParLightWidget.BP_SliderModule_InnerAngle` _asbp_par_light_widget) (`SpotLightComponent.InnerConeAngle` _spotlight)))
    (:`then_3`
      (`/Game/DKW/UI/Module/BP_SliderModule.SetSliderValue` (`/Game/DKW/UI/Light/BP_ParLightWidget.BP_SliderModule_OuterAngle` _asbp_par_light_widget) (`SpotLightComponent.OuterConeAngle` _spotlight)))
    (:`then_4`
      (`/Game/DKW/UI/Module/BP_SliderModule.SetSliderValue` (`/Game/DKW/UI/Light/BP_ParLightWidget.BP_SliderModule_LampTilt` _asbp_par_light_widget) _relativerotation_pitch))
    (:`then_5`
      (`/Game/DKW/UI/Module/BP_SliderModule.SetSliderValue` (`/Game/DKW/UI/Light/BP_ParLightWidget.BP_SliderModule_LampPan` _asbp_par_light_widget) _relativerotation_yaw))
    (:`then_6`
      (set `/Game/DKW/UI/Light/BP_ParLightWidget.isFinishedDefaultVal` true _asbp_par_light_widget))))

(fn `UserConstructionScript`)