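; BP_4x4Frame is a frame light actor pairing a rect light with an emissive fabric mesh driven by a dynamic material.
; Construction and every Tick while LightOn apply intensity, color, barn doors, radius, haze and size to the light, with intensity and size mirrored on the fabric.
; When off, Tick hides the light and zeroes fabric glow.
; OpenAssetPanel spawns a control widget linked to this actor; CloseAssetPanel is empty.
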(event `self.ReceiveBeginPlay`
  (`self.SetOwner` (`GameplayStatics.GetPlayerController` 0)))

(event `self.ReceiveTick`
  (params (DeltaSeconds :type "Float (single-precision)"))
  (if (`self.LightOn`)
    (`self.SetPropertysByParams`)
    (else
      (`self.SetLightOff`))))

(event `self.OpenAssetPanel`
  (params (AssetWithControlPanel :type "Actor Object Reference"))
  (`self.OpenControlWidget`))

(event `self.CloseAssetPanel`
  (params (AssetWithControlPanel :type "Actor Object Reference")))

(fn `OpenControlWidget`
  ;[1 1 1] Create Widget
  (bind _returnvalue (`|CreateWidget` (`self.ControlWidgetSource`)))
  ;[1 1 1] Cast And Save
  (bind _asbp_4x_4frame_light_widget (cast `/Game/DKW/UI/Light/BP_4x4FrameLightWidget` _returnvalue))
  (bind _output_get (set `self.ControlWidget` _asbp_4x_4frame_light_widget))
  ;[1 1 1] Add to View
  (`UserWidget.AddToViewport` _output_get 0)
  (`UserWidget.SetPositionInViewport` (`self.ControlWidget`) (1600.0 50.0) true)
  ;[1 1 1] Control Widget의 AssetRef설정
  (set `/Game/DKW/UI/Light/BP_4x4FrameLightWidget.linkedAsset` self (`self.ControlWidget`)))

(fn `SetLightOff`
  ;[1 1 1] Light On
  (`SceneComponent.SetVisibility` (`self.RectLight`) false false)
  (`MaterialInstanceDynamic.SetScalarParameterValue` (`self.FablicMat`) "Intensity" 0.0))

(fn `SetPropertysByParams`
  (`SceneComponent.SetVisibility` (`self.RectLight`) true false)
  (`|ExecutionSequence`
    (:`then_0`
      (`|ExecutionSequence`
        (:`then_0`
          ;[1 1 1] Intensity / Color
          (`LightComponent.SetIntensity` (`self.RectLight`) (`self.LightIntensity`)))
        (:`then_1`
          (`MaterialInstanceDynamic.SetScalarParameterValue` (`self.FablicMat`) "Intensity" (/ (`self.LightIntensity`) 1000.0)))
        (:`then_2`
          (`LightComponent.SetLightColor` (`self.RectLight`) (`self.LightColor`) true))))
    (:`then_1`
      (`|ExecutionSequence`
        (:`then_0`
          ;[1 1 1] Set Light Area
          (`RectLightComponent.SetBarnDoorAngle` (`self.RectLight`) (`self.LightCoverAngle`)))
        (:`then_1`
          (`RectLightComponent.SetBarnDoorLength` (`self.RectLight`) (`self.LightCoverLength`)))
        (:`then_2`
          (`LocalLightComponent.SetAttenuationRadius` (`self.RectLight`) (`self.LightRadius`)))))
    (:`then_2`
      ;[1 1 1] Haze
      (`LightComponent.SetVolumetricScatteringIntensity` (`self.RectLight`) (`self.LightHazeMult`)))
    (:`then_3`
      (`|ExecutionSequence`
        (:`then_0`
          ;[1 1 1] Set Size
          (`RectLightComponent.SetSourceWidth` (`self.RectLight`) (* (`self.LightWidth`) 100.0)))
        (:`then_1`
          (`RectLightComponent.SetSourceHeight` (`self.RectLight`) (* (`self.LightHeight`) 100.0)))
        (:`then_2`
          (`SceneComponent.SetRelativeScale3D` (`self.FrameLightFabric`) (`KismetMathLibrary.MakeVector` 0.01 (`self.LightWidth`) (`self.LightHeight`))))))))

(fn `UserConstructionScript`
  (bind _framelightfabric (`self.FrameLightFabric`))
  (bind _returnvalue (`KismetMaterialLibrary.CreateDynamicMaterialInstance` "/Game/DKW/Materials/Light/M_RectLight.M_RectLight"))
  (set `self.FablicMat` _returnvalue)
  (`PrimitiveComponent.SetMaterial` _framelightfabric 0 _returnvalue)
  (`SceneComponent.SetRelativeScale3D` _framelightfabric (0.01 1.0 1.0))
  ;[1 1 1] Comment
  (`self.SetPropertysByParams`))