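; BP_SceneCapture2D is an actor, named as a scene capture, that the player nudges sideways with the D key.
; BeginPlay enables input from player controller 0 and prints a leftover debug string.
; D press and release toggle InputRight, and Tick adds the world right vector to the location while it is set.
; Movement is unswept and not scaled by delta time, so speed depends on frame rate.
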(event `self.ReceiveBeginPlay`
  (`self.EnableInput` (`GameplayStatics.GetPlayerController` 0))
  (`KismetSystemLibrary.PrintString` "inputasdjl;fkja;ksdf"))

(event `Key|D`
  (params (Key :type "Key Structure"))
  (:`Pressed`
    (set `self.inputRight` true))
  (:`Released`
    (set `self.inputRight` false)))

(event `self.ReceiveTick`
  (params (DeltaSeconds :type "Float (single-precision)"))
  (if (`self.inputRight`)
    (`self.K2_SetActorLocation` (+ (`self.K2_GetActorLocation`) (`KismetMathLibrary.Vector_Right`)))))

(fn `UserConstructionScript`)