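; Test manager actor that drives gameplay recording and replay from the keyboard.
; On BeginPlay it enables input for player controller 0.
; Keys 1, 2 and 3 cast the game instance to D_GameInstance and call StartRecording, StopRecording and StartReplay respectively.
; Stopping and replaying also print debug strings to the screen.
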(event `self.ReceiveBeginPlay`
  (`self.EnableInput` (`GameplayStatics.GetPlayerController` 0))
  (`KismetSystemLibrary.PrintString` "Hello"))

(event `self.ReceiveTick`
  (params (DeltaSeconds :type "Float (single-precision)")))

(event `Key|One`
  (params (Key :type "Key Structure"))
  (:`Pressed`
    (bind _asd_game_instance (cast `D_GameInstance` (`GameplayStatics.GetGameInstance`)))
    (`D_GameInstance.StartRecording` _asd_game_instance)))

(event `Key|Two`
  (params (Key :type "Key Structure"))
  (:`Pressed`
    (bind _asd_game_instance (cast `D_GameInstance` (`GameplayStatics.GetGameInstance`)))
    (`D_GameInstance.StopRecording` _asd_game_instance)
    (`KismetSystemLibrary.PrintString` "Hello")))

(event `Key|Three`
  (params (Key :type "Key Structure"))
  (:`Pressed`
    (bind _asd_game_instance (cast `D_GameInstance` (`GameplayStatics.GetGameInstance`)))
    (`D_GameInstance.StartReplay` _asd_game_instance)
    (`KismetSystemLibrary.PrintString` "Hello" true true (struct :`R` 0.032125 :`G` 1.0 :`A` 1.0))))

(event `Key|Four`
  (params (Key :type "Key Structure")))

(fn `UserConstructionScript`)