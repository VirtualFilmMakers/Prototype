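; BP_ReplaySpectatorPawn is a spectator pawn for replays that switches the view between camera actors placed in the world.
; On BeginPlay it enables input for player controller 0 and adds the WID_ReplaySpectator widget to the viewport.
; Q caches every CameraActor into an array.
; W sets the view target to the current array entry, then advances the index, wrapping to the first.
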(event `self.ReceiveBeginPlay`
  (bind _returnvalue (`GameplayStatics.GetPlayerController` 0))
  (`|ExecutionSequence`
    (:`then_0`
      (`/Engine/EditorBlueprintResources/StandardMacros.IsValid` _returnvalue
        (:`Is Valid`
          (`self.EnableInput` _returnvalue)
          (`KismetSystemLibrary.PrintString` "controller" true true (struct :`R` 0.143452 :`G` 1.0 :`A` 1.0)))))
    (:`then_1`
      (bind _returnvalue_2 (`|CreateWidget` "/Game/DKW/Blueprints/Record/WID_ReplaySpectator.WID_ReplaySpectator_C" self))
      (`UserWidget.AddToViewport` _returnvalue_2 0))))

(event `Key|Q`
  (params (Key :type "Key Structure"))
  (:`Pressed`
    (bind _outactors (`GameplayStatics.GetAllActorsOfClass` "/Script/Engine.CameraActor"))
    (set `self.Cameras` _outactors)
    (`KismetSystemLibrary.PrintString` "cameras are saved")))

(event `Key|W`
  (params (Key :type "Key Structure"))
  (bind _returnvalue (+ (`self.CamNum`) 1))
  (:`Pressed`
    (`self.SetViewTargetWithBlend` (`GameplayStatics.GetPlayerController` 0) (`|GetArrayItem` (`self.Cameras`) (`self.CamNum`)) 0.0 "VTBlend_Linear" 0.0 false)
    (if (< _returnvalue (`KismetArrayLibrary.Array_Length` (`self.Cameras`)))
      (set `self.CamNum` _returnvalue)
      (else
        (set `self.CamNum` 0)))))

(fn `UserConstructionScript`)