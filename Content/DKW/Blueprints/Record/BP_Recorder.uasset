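; BP_Recorder is a key-driven debug control for starting and stopping replay recording through D_GameInstance.
; Key 1 starts a recording named by SetName, which builds a timestamped "Replay_" string from the current date and time, under the fixed friendly name "Test".
; Key 2 stops the recording, and both keys print on-screen status.
; An unconnected chain for starting replay playback remains in the graph but never runs.
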(event `self.ReceiveBeginPlay`)

(event `Key|One`
  (params (Key :type "Key Structure"))
  (:`Pressed`
    (bind _asd_game_instance (cast `D_GameInstance` (`GameplayStatics.GetGameInstance`)))
    (bind _returnvalue (`self.SetName`))
    (`D_GameInstance.StartRecording` _asd_game_instance _returnvalue "Test")
    (`KismetSystemLibrary.PrintString` "Recording" true true (struct :`R` 1.0 :`G` 0.093222 :`B` 0.083274 :`A` 1.0))))

(event `Key|Two`
  (params (Key :type "Key Structure"))
  (:`Pressed`
    (bind _asd_game_instance (cast `D_GameInstance` (`GameplayStatics.GetGameInstance`)))
    (`D_GameInstance.StopRecording` _asd_game_instance)
    (`KismetSystemLibrary.PrintString` "Stop Record")))

(event `Key|Three`
  (params (Key :type "Key Structure")))

(fn `SetName`
  (returns (ReturnValue :type String))
  (bind (_returnvalue_year _returnvalue_month _returnvalue_day _returnvalue_hour _returnvalue_minute _returnvalue_second) (`KismetMathLibrary.BreakDateTime` (`KismetMathLibrary.Now`)))
  (return (`KismetStringLibrary.Concat_StrStr` "Replay_" (`KismetStringLibrary.Conv_IntToString` _returnvalue_year) "_" (`KismetStringLibrary.Conv_IntToString` _returnvalue_month) "_" (`KismetStringLibrary.Conv_IntToString` _returnvalue_day) "_" (`KismetStringLibrary.Conv_IntToString` _returnvalue_hour) "_" (`KismetStringLibrary.Conv_IntToString` _returnvalue_minute) "_" (`KismetStringLibrary.Conv_IntToString` _returnvalue_second))))