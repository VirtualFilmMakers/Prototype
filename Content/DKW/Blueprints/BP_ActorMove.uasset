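; BP_ActorMove is a keyboard movement test that nudges its owner along the world right axis.
; On BeginPlay it caches the owner as Me and enables input on it for the first player controller.
; A teleports the owner one right-vector step left without sweep and prints debug text.
; D only prints, as the matching rightward move is left unconnected.
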(event `self.ReceiveBeginPlay`
  (bind _output_get (set `self.me` (`self.GetOwner`)))
  (`Actor.EnableInput` _output_get (`GameplayStatics.GetPlayerController` 0))
  (`KismetSystemLibrary.PrintString` "inputasdjl;fkja;ksdf"))

(event `self.ReceiveTick`
  (params (DeltaSeconds :type "Float (single-precision)")))

(event `Key|D`
  (params (Key :type "Key Structure"))
  (:`Pressed`
    (`KismetSystemLibrary.PrintString` "right")))

(event `Key|A`
  (params (Key :type "Key Structure"))
  (bind _me (`self.me`))
  (:`Pressed`
    (`Actor.K2_SetActorLocation` _me (- (`Actor.K2_GetActorLocation` _me) (`KismetMathLibrary.Vector_Right`)) false false)
    (`KismetSystemLibrary.PrintString` "left")))