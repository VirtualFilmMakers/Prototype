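; BP_CineFloatingPlayer is a cinematic player with a CineCamera that zooms smoothly with the mouse wheel.
; Wheel input sets a target focal length as an offset from the current one and prints it to screen.
; Tick eases the camera's focal length toward that target with a fixed-alpha Lerp, so smoothing depends on frame rate.
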(event `self.ReceiveBeginPlay`
  (set `self.TargetFocalLegth` (`CineCameraComponent.CurrentFocalLength` (`self.CineCamera`))))

(event `self.ReceiveTick`
  (params (DeltaSeconds :type "Float (single-precision)"))
  (bind _cinecamera (`self.CineCamera`))
  (set `CineCameraComponent.CurrentFocalLength` (`KismetMathLibrary.Lerp` (`CineCameraComponent.CurrentFocalLength` _cinecamera) (`self.TargetFocalLegth`) 0.1) _cinecamera))

(event `InputAxisKey|MouseWheelAxis`
  (params (AxisValue :type "Float (single-precision)"))
  (bind _output_get (set `self.TargetFocalLegth` (+ (`CineCameraComponent.CurrentFocalLength` (`self.CineCamera`)) (* AxisValue 10.0))))
  (`KismetSystemLibrary.PrintString` (`KismetStringLibrary.Conv_DoubleToString` _output_get)))

(fn `UserConstructionScript`)