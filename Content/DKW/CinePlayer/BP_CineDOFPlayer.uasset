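; Cine camera player Blueprint for switching depth-of-field focus between two characters at runtime.
; On BeginPlay it caches the BP_Natalia and BP_Kristofer actors, which keys 1 and 2 assign as the CineCamera's tracking focus target.
; H toggles the focus method between Manual and Tracking, with debug prints on each input.
; Smooth focal-length zoom by mouse wheel is unfinished: the lerp helper exists, but its calling logic is disconnected.
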(event `self.ReceiveBeginPlay`
  (set `self.TargetFocalLegth` (`CineCameraComponent.CurrentFocalLength` (`self.CineCamera`)))
  (`self.FindSaveActors`))

(event `self.ReceiveTick`
  (params (DeltaSeconds :type "Float (single-precision)")))

(event `Key|H`
  (params (Key :type "Key Structure"))
  (:`Pressed`
    (`/Engine/EditorBlueprintResources/StandardMacros.FlipFlop`
      (:`A`
        (`self.SwitchFocusMode` true)
        (`KismetSystemLibrary.PrintString` "Maual"))
      (:`B`
        (`self.SwitchFocusMode` false)
        (`KismetSystemLibrary.PrintString` "ToFocus")))))

(event `InputAxisKey|MouseWheelAxis`
  (params (AxisValue :type "Float (single-precision)")))

(event `Key|One`
  (params (Key :type "Key Structure"))
  (:`Pressed`
    (`self.SetFocusActor` (`self.Women`))
    (`KismetSystemLibrary.PrintString` "FocusTo Womaen")))

(event `Key|MouseScrollUp`
  (params (Key :type "Key Structure")))

(event `Key|Two`
  (params (Key :type "Key Structure"))
  (:`Pressed`
    (`self.SetFocusActor` (`self.Man`))
    (`KismetSystemLibrary.PrintString` "FocusTo Man")))

(event `Key|LeftShift`
  (params (Key :type "Key Structure")))

(fn `FindSaveActors`
  (`|ExecutionSequence`
    (:`then_0`
      (bind _returnvalue (`GameplayStatics.GetActorOfClass` "/Game/MetaHumans/Kristofer/BP_Kristofer.BP_Kristofer_C"))
      (set `self.Man` _returnvalue))
    (:`then_1`
      (bind _returnvalue_2 (`GameplayStatics.GetActorOfClass` "/Game/MetaHumans/Natalia/BP_Natalia.BP_Natalia_C"))
      (set `self.Women` _returnvalue_2))))

(fn `SetFocusActor`
  (params (FocusActor :type "Actor Object Reference"))
  (bind _cinecamera (`self.CineCamera`))
  (bind _focussettings (`CineCameraComponent.FocusSettings` _cinecamera))
  (set `CineCameraComponent.FocusSettings` (make `CameraFocusSettings` (break `CameraFocusSettings` _focussettings) (`.ManualFocusDistance` (break `CameraFocusSettings` _focussettings)) (make `CameraTrackingFocusSettings` (`|ConvertAsset` FocusActor) (`.RelativeOffset` (break `CameraTrackingFocusSettings` (`.TrackingFocusSettings` (break `CameraFocusSettings` _focussettings)))) (`.bDrawDebugTrackingFocusPoint` (break `CameraTrackingFocusSettings` (`.TrackingFocusSettings` (break `CameraFocusSettings` _focussettings))))) (`.bSmoothFocusChanges` (break `CameraFocusSettings` _focussettings)) (`.FocusSmoothingInterpSpeed` (break `CameraFocusSettings` _focussettings)) (`.FocusOffset` (break `CameraFocusSettings` _focussettings))) _cinecamera))

(fn `SmoothChangeFocalLength`
  (bind _cinecamera (`self.CineCamera`))
  (set `CineCameraComponent.CurrentFocalLength` (`KismetMathLibrary.Lerp` (`CineCameraComponent.CurrentFocalLength` _cinecamera) (`self.TargetFocalLegth`) 0.1) _cinecamera))

(fn `SwitchFocusMode`
  (params (Manual :type Boolean))
  (bind _cinecamera (`self.CineCamera`))
  (bind (_focussettings_focusmethod _focussettings_manualfocusdistance _focussettings_trackingfocussettings _focussettings_bsmoothfocuschanges _focussettings_focussmoothinginterpspeed _focussettings_focusoffset) (break `CameraFocusSettings` (`CineCameraComponent.FocusSettings` _cinecamera)))
  (if Manual
    (set `CineCameraComponent.FocusSettings` (make `CameraFocusSettings` "Manual" _focussettings_manualfocusdistance _focussettings_trackingfocussettings _focussettings_bsmoothfocuschanges _focussettings_focussmoothinginterpspeed _focussettings_focusoffset) _cinecamera)
    (else
      (set `CineCameraComponent.FocusSettings` (make `CameraFocusSettings` "Tracking" _focussettings_manualfocusdistance _focussettings_trackingfocussettings _focussettings_bsmoothfocuschanges _focussettings_focussmoothinginterpspeed _focussettings_focusoffset) _cinecamera))))

(fn `UserConstructionScript`)